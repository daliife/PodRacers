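; EarthquakeEffect is a short-lived spawnable hazard that knocks back POD_PROTOTYPE ships entering its radius.
; When RadiusEffect overlaps a pod, it applies a very large force at the ship mesh's location, opposite the pod's arrow direction.
; The actor destroys itself shortly after that hit, or after a fixed lifetime from spawn.
; Debug prints remain on the delayed overlap path and the component hit event.
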(event OnComponentBeginOverlap(RadiusEffect)
  (params (OverlappedComponent :type Primitive%20Component%20Object%20Reference) (OtherActor :type Actor%20Object%20Reference) (OtherComp :type Primitive%20Component%20Object%20Reference) (OtherBodyIndex :type Integer) (bFromSweep :type Boolean) (SweepResult :type Hit%20Result%20Structure%20%28by%20ref%29))
  (bind _aspod_prototype (Utilities|Casting|CastToPOD_PROTOTYPE OtherActor))
  (Class|PrimitiveComponent|AddForceatLocation (Variables|/Game/Blueprints/PODS/POD_PROTOTYPE.POD_PROTOTYPE_C|GetShipMesh _aspod_prototype) (* (Math|Vector|GetForwardVector (Variables|/Game/Blueprints/PODS/POD_PROTOTYPE.POD_PROTOTYPE_C|GetArrow _aspod_prototype)) -5e+07) (Transformation|GetWorldLocation (Variables|/Game/Blueprints/PODS/POD_PROTOTYPE.POD_PROTOTYPE_C|GetShipMesh _aspod_prototype)) (Utilities|String|StringToName (Utilities|GetObjectName (Variables|/Game/Blueprints/PODS/POD_PROTOTYPE.POD_PROTOTYPE_C|GetShipMesh _aspod_prototype))))
  (Utilities|FlowControl|Delay 1.0)
  (Development|PrintString "Hello")
  (Actor|DestroyActor))

(event OnComponentHit(RadiusEffect)
  (params (HitComponent :type Primitive%20Component%20Object%20Reference) (OtherActor :type Actor%20Object%20Reference) (OtherComp :type Primitive%20Component%20Object%20Reference) (NormalImpulse :type Vector :default "0, 0, 0") (Hit :type Hit%20Result%20Structure%20%28by%20ref%29))
  (Development|PrintString "Hello"))

(event EventBeginPlay
  (Utilities|FlowControl|Delay 6.0)
  (Actor|DestroyActor))

(fn ConstructionScript)