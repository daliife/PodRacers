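; MineProjectile is a spawnable mine with a color-coded pressure plate that explodes after two triggers.
; A state counter advances whenever something leaves the box collider, and once automatically after a long delay from BeginPlay.
; The first step turns the plate's dynamic material from green to yellow with a shutter sound.
; The second fires an explosion impulse with particles and sound, then destroys the actor.
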(event OnComponentEndOverlap(BoxCollider)
  (params (OverlappedComponent :type Primitive%20Component%20Object%20Reference) (OtherActor :type Actor%20Object%20Reference) (OtherComp :type Primitive%20Component%20Object%20Reference) (OtherBodyIndex :type Integer))
  ;[1 1 1] On End Overlap Logic
  (if (< (Variables|Default|GetState) 2)
    (bind _output_get (Variables|Default|SetState (+ (Variables|Default|GetState) 1)))
    (switch int _output_get
      (:0
        (Rendering|Material|SetVectorParameterValue (Variables|Default|GetMaterialReference) "Color" "(R=0.000000,G=1.000000,B=0.000000,A=1.000000)" :!class /Script/Engine.MaterialInstanceDynamic))
      (:1
        (Rendering|Material|SetVectorParameterValue (Variables|Default|GetMaterialReference) "Color" "(R=1.000000,G=1.000000,B=0.000000,A=1.000000)" :!class /Script/Engine.MaterialInstanceDynamic)
        (Audio|PlaySoundatLocation "/Engine/VREditor/Sounds/UI/Camera_Shutter.Camera_Shutter" (Transformation|GetWorldLocation (Variables|Default|GetPressurePlate)) "0, 0, 0" 1.0 1.0 0.0 0 0 0))
      (:2
        (Components|Activation|Deactivate (Variables|Default|GetParticleSystem))
        (Class|RadialForceComponent|FireImpulse (Variables|Default|GetExplosionForce))
        (Effects|SpawnEmitteratLocation "/Game/VFX_Toolkit_V1/ParticleSystems/356Days/Par_WildImpact_01.Par_WildImpact_01" (Transformation|GetWorldLocation (Variables|Default|GetPressurePlate)) "0, 0, 0" "5.000000,5.000000,5.000000")
        (Audio|PlaySoundatLocation "/Game/StarterContent/Audio/Explosion01.Explosion01" (Transformation|GetWorldLocation (Variables|Default|GetBoxCollider)) "0, 0, 0" 1.0 1.0 0.0 0 0 0)
        (Utilities|FlowControl|Delay 0.2)
        (Actor|DestroyActor)))))

(event EventBeginPlay
  ;[1 1 1] Initialization
  (Variables|Default|SetState 0)
  (bind _returnvalue (Rendering|Material|CreateDynamicMaterialInstance (Variables|Default|GetPressurePlate) 0 "/Game/Materials/mat_projectile.mat_projectile" "None" :!class /Script/Engine.PrimitiveComponent))
  (bind _output_get (Variables|Default|SetMaterialReference _returnvalue))
  (Rendering|Material|SetVectorParameterValue _output_get "Color" "(R=0.000000,G=1.000000,B=0.000000,A=1.000000)" :!class /Script/Engine.MaterialInstanceDynamic)
  (Utilities|FlowControl|Delay 6e+01)
  ;[1 1 1] On End Overlap Logic
  (bind _output_get_2 (Variables|Default|SetState (+ (Variables|Default|GetState) 1)))
  (switch int _output_get_2
    (:0
      (Rendering|Material|SetVectorParameterValue (Variables|Default|GetMaterialReference) "Color" "(R=0.000000,G=1.000000,B=0.000000,A=1.000000)" :!class /Script/Engine.MaterialInstanceDynamic))
    (:1
      (Rendering|Material|SetVectorParameterValue (Variables|Default|GetMaterialReference) "Color" "(R=1.000000,G=1.000000,B=0.000000,A=1.000000)" :!class /Script/Engine.MaterialInstanceDynamic)
      (Audio|PlaySoundatLocation "/Engine/VREditor/Sounds/UI/Camera_Shutter.Camera_Shutter" (Transformation|GetWorldLocation (Variables|Default|GetPressurePlate)) "0, 0, 0" 1.0 1.0 0.0 0 0 0))
    (:2
      (Components|Activation|Deactivate (Variables|Default|GetParticleSystem))
      (Class|RadialForceComponent|FireImpulse (Variables|Default|GetExplosionForce))
      (Effects|SpawnEmitteratLocation "/Game/VFX_Toolkit_V1/ParticleSystems/356Days/Par_WildImpact_01.Par_WildImpact_01" (Transformation|GetWorldLocation (Variables|Default|GetPressurePlate)) "0, 0, 0" "5.000000,5.000000,5.000000")
      (Audio|PlaySoundatLocation "/Game/StarterContent/Audio/Explosion01.Explosion01" (Transformation|GetWorldLocation (Variables|Default|GetBoxCollider)) "0, 0, 0" 1.0 1.0 0.0 0 0 0)
      (Utilities|FlowControl|Delay 0.2)
      (Actor|DestroyActor))))

(fn ConstructionScript)