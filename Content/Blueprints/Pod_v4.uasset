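; Pod Blueprint that keeps its Cube component raised above surfaces beneath it.
; Each Tick, a debug-drawn Visibility line trace runs from the Cube along its negative up vector for DesiredElevation.
; A closer hit nudges the Cube by a fixed, unswept step using its up vector as a relative offset.
; The step is not scaled by delta time, and nothing lowers the Cube.
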(event EventTick
  (params (DeltaSeconds :type Float%20%28single-precision%29))
  (bind _cube (Variables|Default|GetCube))
  (bind _cube_2 (Variables|Default|GetCube))
  (bind _returnvalue (Transformation|GetWorldLocation _cube))
  (bind (_outhit _returnvalue_2) (Collision|LineTraceByChannel _returnvalue (+ _returnvalue (* (Math|Vector|GetUpVector _cube) (* (Variables|Default|GetDesiredElevation) -1.0))) "TraceTypeQuery1" false 0 "ForDuration" true "(R=1.000000,G=0.000000,B=0.000000,A=1.000000)" "(R=0.000000,G=1.000000,B=0.000000,A=1.000000)" 0.5))
  (if _returnvalue_2
    (if (< (.Distance (Collision|BreakHitResult _outhit)) (Variables|Default|GetDesiredElevation))
      (Transformation|AddRelativeLocation _cube_2 (* (Math|Vector|GetUpVector _cube_2) 1.0) false false))))

(fn ConstructionScript)