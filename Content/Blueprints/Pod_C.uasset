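; Pod_C is a ship pod Blueprint whose ultimate ability is an instant forward jump.
; Pressing UltimateAbility offsets the ship mesh and the front, left and right sphere colliders a long way along the StabilizationPlane's forward vector, plus a slight lift along its up vector.
; The move teleports without sweeping, skipping collision along the path.
; Unconnected nodes that re-set each collider's relative location never run.
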(event EventBeginPlay
  (|CallParentFunction) ; This node is disabled and will not be called.\nDrag off pins to build functionality.
)

(event Collision|EventActorBeginOverlap
  (params (OtherActor :type Actor%20Object%20Reference)))

(event EventTick
  (params (DeltaSeconds :type Float%20%28single-precision%29))
  (|CallParentFunction DeltaSeconds) ; This node is disabled and will not be called.\nDrag off pins to build functionality.
)

(event Input|ActionEvents|InputActionUltimateAbility
  (params (Key :type Key%20Structure))
  (bind _stabilizationplane (Variables|Default|GetStabilizationPlane))
  (:Pressed
    (Transformation|AddWorldOffset (Variables|Default|GetRight_Sphere_Collider) (+ (* (Math|Vector|GetForwardVector _stabilizationplane) 5e+03) (* (Math|Vector|GetUpVector _stabilizationplane) 5e+01)) false true)))

(fn ConstructionScript
  (|CallParentFunction))