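; Mine projectile actor with a pressure plate that escalates from green to yellow to red, then explodes.
; Each box overlap advances the state, as does a one-time 60-second timer from BeginPlay, recoloring a dynamic material and playing a warning sound.
; At red, a short countdown precedes a radial impulse, explosion particles and sound, then the plate hides and the actor destroys itself.
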(event OnComponentBeginOverlap(BoxCollider)
  (params (OverlappedComponent :type Primitive%20Component%20Object%20Reference) (OtherActor :type Actor%20Object%20Reference) (OtherComp :type Primitive%20Component%20Object%20Reference) (OtherBodyIndex :type Integer) (bFromSweep :type Boolean) (SweepResult :type Hit%20Result%20Structure%20%28by%20ref%29))
  (if (< (Variables|Default|GetState) 2)
    (bind _output_get (Variables|Default|SetState (+ (Variables|Default|GetState) 1) :!label _label))
    (switch int _output_get
      (:0
        (Rendering|Material|SetVectorParameterValue (stale EventBeginPlay _output_get) "Color" "(R=0.000000,G=1.000000,B=0.000000,A=1.000000)" :!class /Script/Engine.MaterialInstanceDynamic)
        (Utilities|FlowControl|Delay 6e+01)
        (goto _label))
      (:1
        (Rendering|Material|SetVectorParameterValue (Variables|Default|GetMaterialReference) "Color" "(R=1.000000,G=1.000000,B=0.000000,A=1.000000)" :!class /Script/Engine.MaterialInstanceDynamic)
        (Audio|PlaySoundatLocation "/Engine/VREditor/Sounds/UI/Camera_Shutter.Camera_Shutter" (Transformation|GetWorldLocation (Variables|Default|GetPressurePlate)) "0, 0, 0" 1.0 1.0 0.0 0 0 0))
      (:2
        (Rendering|Material|SetVectorParameterValue (Variables|Default|GetMaterialReference) "Color" "(R=1.000000,G=0.000000,B=0.000000,A=1.000000)" :!class /Script/Engine.MaterialInstanceDynamic)
        (Audio|PlaySoundatLocation "/Game/Sounds/SFX/bombcountdown.bombcountdown" (Transformation|GetWorldLocation (Variables|Default|GetPressurePlate)) "0, 0, 0" 1.0 1.0 0.0 0 0 0)
        (Utilities|FlowControl|Delay 2.0)
        (Class|RadialForceComponent|FireImpulse (Variables|Default|GetExplosionForce))
        (Effects|SpawnEmitteratLocation "/Game/StarterContent/Particles/P_Explosion.P_Explosion" (Transformation|GetWorldLocation (Variables|Default|GetPressurePlate)) "0, 0, 0" "5.000000,5.000000,5.000000")
        (Audio|PlaySoundatLocation "/Game/StarterContent/Audio/Explosion01.Explosion01" "0, 0, 0" "0, 0, 0" 1.0 1.0 0.0 0 0 0)
        (Rendering|SetVisibility (Variables|Default|GetPressurePlate) false false)
        (Utilities|FlowControl|Delay 1.0)
        (Actor|DestroyActor)))))

(event EventBeginPlay
  (bind _returnvalue (Rendering|Material|CreateDynamicMaterialInstance (Variables|Default|GetPressurePlate) 0 "/Game/Materials/mat_projectile.mat_projectile" "None" :!class /Script/Engine.PrimitiveComponent))
  (Variables|Default|SetState 0)
  (bind _output_get (Variables|Default|SetMaterialReference _returnvalue))
  (Rendering|Material|SetVectorParameterValue _output_get "Color" "(R=0.000000,G=1.000000,B=0.000000,A=1.000000)" :!class /Script/Engine.MaterialInstanceDynamic :!label _label)
  (Utilities|FlowControl|Delay 6e+01)
  (bind _output_get_2 (Variables|Default|SetState (+ (Variables|Default|GetState) 1)))
  (switch int _output_get_2
    (:0
      (goto _label))
    (:1
      (Rendering|Material|SetVectorParameterValue (Variables|Default|GetMaterialReference) "Color" "(R=1.000000,G=1.000000,B=0.000000,A=1.000000)" :!class /Script/Engine.MaterialInstanceDynamic)
      (Audio|PlaySoundatLocation "/Engine/VREditor/Sounds/UI/Camera_Shutter.Camera_Shutter" (Transformation|GetWorldLocation (Variables|Default|GetPressurePlate)) "0, 0, 0" 1.0 1.0 0.0 0 0 0))
    (:2
      (Rendering|Material|SetVectorParameterValue (Variables|Default|GetMaterialReference) "Color" "(R=1.000000,G=0.000000,B=0.000000,A=1.000000)" :!class /Script/Engine.MaterialInstanceDynamic)
      (Audio|PlaySoundatLocation "/Game/Sounds/SFX/bombcountdown.bombcountdown" (Transformation|GetWorldLocation (Variables|Default|GetPressurePlate)) "0, 0, 0" 1.0 1.0 0.0 0 0 0)
      (Utilities|FlowControl|Delay 2.0)
      (Class|RadialForceComponent|FireImpulse (Variables|Default|GetExplosionForce))
      (Effects|SpawnEmitteratLocation "/Game/StarterContent/Particles/P_Explosion.P_Explosion" (Transformation|GetWorldLocation (Variables|Default|GetPressurePlate)) "0, 0, 0" "5.000000,5.000000,5.000000")
      (Audio|PlaySoundatLocation "/Game/StarterContent/Audio/Explosion01.Explosion01" "0, 0, 0" "0, 0, 0" 1.0 1.0 0.0 0 0 0)
      (Rendering|SetVisibility (Variables|Default|GetPressurePlate) false false)
      (Utilities|FlowControl|Delay 1.0)
      (Actor|DestroyActor))))

(fn ConstructionScript)