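; Race manager that fills the starting grid by spawning pods above the race placeholders at match start.
; On BeginPlay it reads enemy count, chosen pod and ability setting from the settings game instance.
; A random slot gets the player's pod type, possessed by player controller 0; other slots get random pod types with AI enabled.
; Spawning stops once the enemy count plus the player is placed.
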(event EventBeginPlay
  (bind _assettings_game_instance (Utilities|Casting|CastToSettingsGameInstance (Game|GetGameInstance)))
  (Variables|Default|SetNumPods (Variables|/Game/GameModes/SettingsGameInstance.SettingsGameInstance_C|GetNumEnemies _assettings_game_instance))
  (Variables|Default|SetPlayersChoice (Variables|/Game/GameModes/SettingsGameInstance.SettingsGameInstance_C|GetIDPod _assettings_game_instance))
  (Variables|Default|SetUseAbility (Variables|/Game/GameModes/SettingsGameInstance.SettingsGameInstance_C|GetUseAbilities _assettings_game_instance))
  (CallFunction|SpawnPods))

(fn ConstructionScript)

(fn SpawnPods
  (bind _returnvalue (Game|GetPlayerController 0))
  (bind _useability (Variables|Default|GetUseAbility))
  (Variables|Default|SetPlayerSpawnPos (Math|Random|RandomIntegerinRange 0 (Variables|Default|GetNumPods)))
  (bind (_array_element _array_index) (Utilities|Array|ForEachLoopwithBreak (Variables|Default|GetRacePlaceholders) :!label _label)
    (:LoopBody
      (switch int (select (== (Variables|Default|GetPlayerSpawnPos) _array_index) (Variables|Default|GetPlayersChoice) (Math|Random|RandomIntegerinRange 0 2))
        (:0
          (bind _returnvalue_2 (Game|SpawnActorfromClass "/Game/Blueprints/PODS/Pod_A.Pod_A_C" (Math|Transform|MakeTransform (+ (.Location (Math|Transform|BreakTransform (Transformation|GetWorldTransform (Variables|/Game/Blueprints/GAMELOGIC/PodSpawnPlaceholder.PodSpawnPlaceholder_C|GetDefaultSceneRoot _array_element)))) "0, 0,150.000000") (.Rotation (Math|Transform|BreakTransform (Transformation|GetWorldTransform (Variables|/Game/Blueprints/GAMELOGIC/PodSpawnPlaceholder.PodSpawnPlaceholder_C|GetDefaultSceneRoot _array_element))))) "Undefined" 0 0))
          (Variables|/Game/Blueprints/PODS/POD_PROTOTYPE.POD_PROTOTYPE_C|SetUseAbilities _returnvalue_2 _useability)
          (Variables|/Game/Blueprints/PODS/POD_PROTOTYPE.POD_PROTOTYPE_C|SetUseIA _returnvalue_2 (not (== (Variables|Default|GetPlayerSpawnPos) _array_index)))
          (if (== (Variables|Default|GetPlayerSpawnPos) _array_index)
            (Pawn|Possess _returnvalue _returnvalue_2)))
        (:1
          (bind _returnvalue_3 (Game|SpawnActorfromClass "/Game/Blueprints/PODS/Pod_B.Pod_B_C" (Math|Transform|MakeTransform (+ (.Location (Math|Transform|BreakTransform (Transformation|GetWorldTransform (Variables|/Game/Blueprints/GAMELOGIC/PodSpawnPlaceholder.PodSpawnPlaceholder_C|GetDefaultSceneRoot _array_element)))) "0, 0,150.000000") (.Rotation (Math|Transform|BreakTransform (Transformation|GetWorldTransform (Variables|/Game/Blueprints/GAMELOGIC/PodSpawnPlaceholder.PodSpawnPlaceholder_C|GetDefaultSceneRoot _array_element))))) "Undefined" 0 0))
          (Variables|/Game/Blueprints/PODS/POD_PROTOTYPE.POD_PROTOTYPE_C|SetUseAbilities _returnvalue_3 _useability)
          (Variables|/Game/Blueprints/PODS/POD_PROTOTYPE.POD_PROTOTYPE_C|SetUseIA _returnvalue_3 (not (== (Variables|Default|GetPlayerSpawnPos) _array_index)))
          (if (== (Variables|Default|GetPlayerSpawnPos) _array_index)
            (Pawn|Possess _returnvalue _returnvalue_3)))
        (:2
          (bind _returnvalue_4 (Game|SpawnActorfromClass "/Game/Blueprints/PODS/Pod_C.Pod_C_C" (Math|Transform|MakeTransform (+ (.Location (Math|Transform|BreakTransform (Transformation|GetWorldTransform (Variables|/Game/Blueprints/GAMELOGIC/PodSpawnPlaceholder.PodSpawnPlaceholder_C|GetDefaultSceneRoot _array_element)))) "0, 0,150.000000") (.Rotation (Math|Transform|BreakTransform (Transformation|GetWorldTransform (Variables|/Game/Blueprints/GAMELOGIC/PodSpawnPlaceholder.PodSpawnPlaceholder_C|GetDefaultSceneRoot _array_element))))) "Undefined" 0 0))
          (Variables|/Game/Blueprints/PODS/POD_PROTOTYPE.POD_PROTOTYPE_C|SetUseAbilities _returnvalue_4 _useability)
          (Variables|/Game/Blueprints/PODS/POD_PROTOTYPE.POD_PROTOTYPE_C|SetUseIA _returnvalue_4 (not (== (Variables|Default|GetPlayerSpawnPos) _array_index)))
          (if (== (Variables|Default|GetPlayerSpawnPos) _array_index)
            (Pawn|Possess _returnvalue _returnvalue_4))))
      (if (>= _array_index (Variables|Default|GetNumPods))
        (goto _label Break)))))