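; Missile projectile actor that explodes with a radial impulse, particle effect and sound, then destroys itself.
; Its first hit on a physics-simulating component stops movement and starts the fuse; a 60-second timeout after BeginPlay also starts it.
; The fuse is a timeline that blends the sphere's dynamic material from green to red and detonates on finish.
; Hits on non-simulating components only print a debug message.
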(event OnComponentHit(CollisionComponent)
  (params (HitComponent :type Primitive%20Component%20Object%20Reference) (OtherActor :type Actor%20Object%20Reference) (OtherComp :type Primitive%20Component%20Object%20Reference) (NormalImpulse :type Vector :default "0, 0, 0") (Hit :type Hit%20Result%20Structure%20%28by%20ref%29))
  (bind _explosionforce (Variables|Default|GetExplosionForce))
  (bind _returnvalue (Transformation|GetWorldLocation _explosionforce))
  ;[1 1 1] Explode on contact
  (if (Physics|IsSimulatingPhysics OtherComp "None")
    (Utilities|FlowControl|DoOnce false
      (:Completed
        (Components|Movement|StopMovementImmediately (Variables|Default|GetProjectileMovement))
        (bind _newtrack_0 (Timeline|ColorTimeline Play)
          (:Update
            (Rendering|Material|SetVectorParameterValue (Variables|Default|GetMaterialReference) "Color" (Math|Color|Lerp(LinearColor) "(R=0.000000,G=1.000000,B=0.000000,A=1.000000)" "(R=1.000000,G=0.000000,B=0.000000,A=1.000000)" _newtrack_0) :!class /Script/Engine.MaterialInstanceDynamic))
          (:Finished
            (Class|RadialForceComponent|FireImpulse _explosionforce)
            (Effects|SpawnEmitteratLocation "/Game/StarterContent/Particles/P_Explosion.P_Explosion" _returnvalue)
            (Audio|PlaySoundatLocation "/Game/StarterContent/Audio/Explosion01.Explosion01" _returnvalue "0, 0, 0" 1.0 1.0 0.0 0 0 0)
            (Actor|DestroyActor)))))
    (else
      (Development|PrintString "No physics simulation activated on actor"))))

(event EventBeginPlay
  (bind _explosionforce (Variables|Default|GetExplosionForce))
  (bind _returnvalue (Transformation|GetWorldLocation _explosionforce))
  ;[1 1 1] Missile timeout
  (bind _returnvalue_2 (Rendering|Material|CreateDynamicMaterialInstance (Variables|Default|GetSphere) 0 "/Game/Materials/mat_projectile.mat_projectile" "None" :!class /Script/Engine.PrimitiveComponent))
  (Variables|Default|SetMaterialReference _returnvalue_2)
  (Utilities|FlowControl|Delay 6e+01)
  ;[1 1 1] Explode on contact
  (bind _newtrack_0 (Timeline|ColorTimeline Play)
    (:Update
      (Rendering|Material|SetVectorParameterValue (Variables|Default|GetMaterialReference) "Color" (Math|Color|Lerp(LinearColor) "(R=0.000000,G=1.000000,B=0.000000,A=1.000000)" "(R=1.000000,G=0.000000,B=0.000000,A=1.000000)" _newtrack_0) :!class /Script/Engine.MaterialInstanceDynamic))
    (:Finished
      (Class|RadialForceComponent|FireImpulse _explosionforce)
      (Effects|SpawnEmitteratLocation "/Game/StarterContent/Particles/P_Explosion.P_Explosion" _returnvalue)
      (Audio|PlaySoundatLocation "/Game/StarterContent/Audio/Explosion01.Explosion01" _returnvalue "0, 0, 0" 1.0 1.0 0.0 0 0 0)
      (Actor|DestroyActor))))

(fn ConstructionScript)