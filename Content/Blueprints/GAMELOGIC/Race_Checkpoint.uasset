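; Race checkpoint actor that registers when a player-driven pod passes through it in the correct direction.
; When a POD_PROTOTYPE leaves the Trigger, it ignores AI pods and uses a dot product of velocity and the Arrow's forward vector to confirm direction.
; A valid pass calls CheckpointCleared with its checkpoint number, hides the particle effect and disables trigger overlaps so it fires only once.
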(event OnComponentEndOverlap(Trigger)
  (params (OverlappedComponent :type Primitive%20Component%20Object%20Reference) (OtherActor :type Actor%20Object%20Reference) (OtherComp :type Primitive%20Component%20Object%20Reference) (OtherBodyIndex :type Integer))
  ;[1 1 1] Checkpoint System - Cleared when overlap end
  (bind _aspod_prototype (Utilities|Casting|CastToPOD_PROTOTYPE OtherActor))
  (if (and (not (Variables|/Game/Blueprints/PODS/POD_PROTOTYPE.POD_PROTOTYPE_C|GetUseIA _aspod_prototype)) (> (Math|Vector|DotProduct (Transformation|GetVelocity _aspod_prototype) (Math|Rotator|GetRotationXVector (Transformation|GetWorldRotation (Variables|Default|GetArrow)))) 0.0))
    (Default|CallCheckpointCleared (Variables|Default|GetCheckpointNumber))
    (Development|SetHiddeninGame (Variables|Default|GetParticleSystem) true false)
    (Variables|/Script/Engine.PrimitiveComponent|SetbGenerateOverlapEvents (Variables|Default|GetTrigger) false)))

(fn ConstructionScript)