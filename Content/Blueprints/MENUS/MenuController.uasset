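; Menu controller that moves the player's view between main, map, settings, about, tutorial and pod cameras using eased view-target blends.
; BeginPlay shows the main camera and caches menu widgets; Tick rebinds menu, back and select widget events every frame.
; An integer State tracks depth: back steps toward the main camera, while select advances to the pod camera, then opens LevelWithAssets.
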(event Custom|GoBack
  ;[1 1 1] Event tick
  (switch int (Variables|Default|GetState)
    (:1
      (CallFunction|GotoCam (Variables|CamReferences|GetMainCam) true))
    (:2
      (CallFunction|GotoCam (Variables|CamReferences|GetMapCam) true)))
  (Variables|Default|SetState (- (Variables|Default|GetState) 1)))

(event Custom|GoSelect
  ;[1 1 1] Event tick
  (switch int (Variables|Default|GetState)
    (:0
      (CallFunction|GotoCam (Variables|CamReferences|GetPodCam) true :!label _label)
      (Variables|Default|SetState 2))
    (:1
      (goto _label))
    (:2
      (Game|OpenLevel(byName) "LevelWithAssets"))))

(event Custom|GoPlay
  ;[1 1 1] Event tick
  (CallFunction|GotoCam (Variables|CamReferences|GetMapCam) true)
  (Variables|Default|SetState 1))

(event Custom|GoSettings
  ;[1 1 1] Event tick
  (CallFunction|GotoCam (Variables|CamReferences|GetSettingsCam) true))

(event Custom|GoAbout
  ;[1 1 1] Event tick
  (CallFunction|GotoCam (Variables|CamReferences|GetAboutCam) true))

(event Custom|GoTutorial
  ;[1 1 1] Event tick
  (CallFunction|GotoCam (Variables|CamReferences|GetTutorialCam) true))

(event EventTick
  (params (DeltaSeconds :type Float%20%28single-precision%29))
  ;[1 1 1] Event tick
  (EventDispatchers|BindEventtoGoPlay (Variables|WidgetReference|GetMenuReference) (delegate Custom|GoPlay))
  (EventDispatchers|BindEventtoGoSettings (Variables|WidgetReference|GetMenuReference) (delegate Custom|GoSettings))
  (EventDispatchers|BindEventtoGoAbout (Variables|WidgetReference|GetMenuReference) (delegate Custom|GoAbout))
  (EventDispatchers|BindEventtoGoTutorial (Variables|WidgetReference|GetMenuReference) (delegate Custom|GoTutorial))
  (for _array_element (Variables|WidgetReference|GetBackReference)
    (EventDispatchers|BindEventtoGoMenu _array_element (delegate Custom|GoBack)))
  (for _array_element_2 (Variables|WidgetReference|GetSelectReference)
    (EventDispatchers|BindEventtoGoSelect _array_element_2 (delegate Custom|GoSelect))))

(event EventBeginPlay
  ;[1 1 1] Event Begin Play
  (CallFunction|GotoCam (Variables|CamReferences|GetMainCam) true)
  (Utilities|FlowControl|Sequence
    (:then_0
      (bind _foundwidgets (Widget|GetAllWidgetsOfClass "/Game/Widgets/Menus/MenuWidget.MenuWidget_C" false))
      (Variables|WidgetReference|SetMenuReference _foundwidgets))
    (:then_1
      (bind _foundwidgets_2 (Widget|GetAllWidgetsOfClass "/Game/Widgets/Menus/SettingWidget.SettingWidget_C" false))
      (Variables|WidgetReference|SetSettingsReference _foundwidgets_2))
    (:then_2
      (bind _foundwidgets_3 (Widget|GetAllWidgetsOfClass "/Game/Widgets/Menus/MapWidget.MapWidget_C" false))
      (Variables|WidgetReference|SetLevelsReference _foundwidgets_3))
    (:then_3
      (bind _foundwidgets_4 (Widget|GetAllWidgetsOfClass "/Game/Widgets/Menus/BackWidget.BackWidget_C" false))
      (Variables|WidgetReference|SetBackReference _foundwidgets_4))
    (:then_4
      (bind _foundwidgets_5 (Widget|GetAllWidgetsOfClass "/Game/Widgets/Menus/SelectWidget.SelectWidget_C" false))
      (Variables|WidgetReference|SetSelectReference _foundwidgets_5))))

(fn ConstructionScript)

(fn GotoCam
  (params (NewCamera :type Camera%20Actor%20Object%20Reference) (withTransition :type Boolean))
  ;[1 1 1] Animation to selected cam
  (Game|Player|SetViewTargetwithBlend (Game|GetPlayerController 0) NewCamera (select withTransition (Variables|Default|GetTransitionSpeed) 0.0) "VTBlend_EaseInOut" 5.0 false))

(fn UpdateEventCalls)