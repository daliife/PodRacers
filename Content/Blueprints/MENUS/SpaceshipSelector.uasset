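; Menu actor for selecting a spaceship, showing a pod mesh that spins around its yaw axis alongside a widget.
; UpdatePodMesh looks up a row ID in the PodData table, sets the mesh and passes the pod name to the ShipSelectorWidget, starting with row "0" on BeginPlay.
; Tick plays the Sin timeline, whose update rotates the mesh by delta time and RotationSpeed, without reading a curve value.
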(event EventTick
  (params (DeltaSeconds :type Float%20%28single-precision%29))
  (Timeline|sin Play
    (:Update
      (Transformation|AddLocalRotation (Variables|Default|GetStaticMesh) (Math|Rotator|MakeRotator 0.0 0.0 (* DeltaSeconds (Variables|Default|GetRotationSpeed))) false false))))

(event EventBeginPlay
  (CallFunction|UpdatePodMesh "0"))

(fn ConstructionScript)

(fn UpdatePodMesh
  (params (ID :type Name))
  (bind _returnvalue (Utilities|GetDataTableRow "/Game/Data/PodData.PodData" ID)
    (:then
      (Components|StaticMesh|SetStaticMesh (Variables|Default|GetStaticMesh) (.PodMesh (Utilities|Struct|BreakPodStruct _returnvalue)))
      (bind _asship_selector_widget (Utilities|Casting|CastToShipSelectorWidget (UserInterface|GetUserWidgetObject (Variables|Default|GetWidget))))
      (Variables|/Game/Widgets/Menus/ShipSelectorWidget.ShipSelectorWidget_C|SetPodName _asship_selector_widget (Utilities|String|ToString(Text) (.PodName (Utilities|Struct|BreakPodStruct _returnvalue)))))
    (:RowNotFound
      (Development|PrintString "NOT FOUND"))))