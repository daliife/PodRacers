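; Player-controlled hover pod Blueprint that drives a physics body, orbit/zoom camera and viewport HUD widget.
; Each Tick it stores speed and traces world-down from four corner constraints, placing supports at the ground hit or OptimalZ below.
; The body trace's surface normal is passed along but unused.
; Input sets forward and turn thruster strength, while Turbo and Brake flip-flop boost and linear damping on press and release.
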(event EventBeginPlay
  (bind _returnvalue (UserInterface|CreateWidget "/Game/Sprites/hud_player_right.hud_player_right_C" (Game|GetPlayerController 0)))
  (UserInterface|Viewport|AddtoViewport _returnvalue 0))

(event EventTick
  (params (DeltaSeconds :type Float%20%28single-precision%29))
  (bind _mainbody (Variables|Default|GetMainBody))
  (bind _returnvalue (Transformation|GetWorldLocation _mainbody))
  (Variables|Default|SetCurrSpeed (Math|Float|Sqrt (Math|Vector|VectorLengthSquared (Transformation|GetComponentVelocity (Variables|Default|GetMainBody)))))
  (bind _outhit (Collision|LineTraceByChannel _returnvalue (+ _returnvalue (* (Math|Vector|GetUpVector _mainbody) -3e+02)) "TraceTypeQuery1" false 0 "None" true "(R=0.000000,G=1.000000,B=0.111239,A=1.000000)" "(R=1.000000,G=0.000000,B=0.511419,A=1.000000)"))
  (CallFunction|SetSupportLocations (Variables|Default|GetBackLeftCon) (Variables|Default|GetBackLeftSup) (.ImpactNormal (Collision|BreakHitResult _outhit)))
  (CallFunction|SetSupportLocations (Variables|Default|GetBackRightCon) (Variables|Default|GetBackRightSup) (.ImpactNormal (Collision|BreakHitResult _outhit)))
  (CallFunction|SetSupportLocations (Variables|Default|GetFrontRightCon) (Variables|Default|GetFrontRightSup) (.ImpactNormal (Collision|BreakHitResult _outhit)))
  (CallFunction|SetSupportLocations (Variables|Default|GetFrontLeftCon) (Variables|Default|GetFrontLeftSup) (.ImpactNormal (Collision|BreakHitResult _outhit))))

(event Input|ActionEvents|InputActionBrake
  (params (Key :type Key%20Structure))
  (:Pressed
    (Utilities|FlowControl|FlipFlop :!label _label
      (:A
        (Class|PrimitiveComponent|SetLinearDamping (Variables|Default|GetMainBody) 1.0))
      (:B
        (Class|PrimitiveComponent|SetLinearDamping (Variables|Default|GetMainBody) 0.1))))
  (:Released
    (goto _label)))

(event Input|ActionEvents|InputActionTurbo
  (params (Key :type Key%20Structure))
  (:Pressed
    (Utilities|FlowControl|FlipFlop :!label _label
      (:A
        (Variables|Default|SetThrustForwardBoost 4.0))
      (:B
        (Variables|Default|SetThrustForwardBoost 1.0))))
  (:Released
    (goto _label)))

(event Input|AxisEvents|InputAxisMoveForward
  (params (AxisValue :type Float%20%28single-precision%29))
  (Variables|/Script/Engine.PhysicsThrusterComponent|SetThrustStrength (Variables|Default|GetForwardThrust) (* AxisValue (* (Variables|Default|GetThrustForwardForce) (Variables|Default|GetThrustForwardBoost)))))

(event Input|AxisEvents|InputAxisMoveRight
  (params (AxisValue :type Float%20%28single-precision%29))
  (Variables|/Script/Engine.PhysicsThrusterComponent|SetThrustStrength (Variables|Default|GetTurnThrust) (* AxisValue 1e+05)))

(event Input|AxisEvents|InputAxisTurnRate
  (params (AxisValue :type Float%20%28single-precision%29))
  (Transformation|AddRelativeRotation (Variables|Default|GetSpringArm) (Math|Rotator|MakeRotator 0.0 0.0 (* AxisValue (Variables|Default|GetCameraVelocity))) false false))

(event Input|AxisEvents|InputAxisLookUpRate
  (params (AxisValue :type Float%20%28single-precision%29))
  (Transformation|AddRelativeRotation (Variables|Default|GetSpringArm) (Math|Rotator|MakeRotator 0.0 (* AxisValue (Variables|Default|GetCameraVelocity)) 0.0) false false))

(event Input|MouseEvents|MouseWheelAxis
  (params (AxisValue :type Float%20%28single-precision%29))
  (bind _springarm (Variables|Default|GetSpringArm))
  (Variables|/Script/Engine.SpringArmComponent|SetTargetArmLength _springarm (+ (* AxisValue -5.0) (Variables|/Script/Engine.SpringArmComponent|GetTargetArmLength _springarm))))

(fn ConstructionScript)

(fn SetSupportLocations
  (params (Constraint :type Physics%20Constraint%20Component%20Object%20Reference) (Support :type Static%20Mesh%20Component%20Object%20Reference) (UpVector :type Vector))
  (bind _returnvalue (Transformation|GetWorldLocation Constraint))
  (bind _optimalz (Variables|Default|GetOptimalZ))
  (bind _returnvalue_2 (* "0, 0,1.000000" _optimalz))
  (bind _returnvalue_3 (- _returnvalue _returnvalue_2))
  (bind (_outhit _returnvalue_4) (Collision|LineTraceByChannel _returnvalue _returnvalue_3 "TraceTypeQuery1" false 0 "None" true "(R=1.000000,G=0.000000,B=0.000000,A=1.000000)" "(R=0.000000,G=1.000000,B=0.000000,A=1.000000)" 0.1))
  (if _returnvalue_4
    (Transformation|SetWorldLocation Support (.Location (Collision|BreakHitResult _outhit)) false false)
    (else
      (Transformation|SetWorldLocation Support _returnvalue_3 false false)))
  (return))