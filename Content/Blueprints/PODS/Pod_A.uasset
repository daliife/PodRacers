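; Pod_A is a racing pod variant with a forward missile ability and an invisibility ultimate.
; Invisibility swaps the mesh to a stealth material, toggling particles and playing sounds.
; AI checks each tick, firing at nearby pods ahead via a dot product and cloaking near rivals; triggered abilities get effectiveness-based AI delays.
; Respawn spawns a fresh Pod_A, copies race state and repossesses it for human players.
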(event EventBeginPlay
  ;[1 1 1] Event BeginPlay
  (|CallParentFunction)
  (CallFunction|InitStatsValues "POD_A"))

(event EventRespawn
  (params (respawnLocation :type Transform) (isIA :type Boolean) (OldActor :type POD%20PROTOTYPE%20Object%20Reference))
  ;[1 1 1] Respawn Logic
  (bind _returnvalue (Game|SpawnActorfromClass "Pod_A_C" respawnLocation "AdjustIfPossibleButAlwaysSpawn" 0 0))
  (Variables|/Game/Blueprints/PODS/POD_PROTOTYPE.POD_PROTOTYPE_C|SetUseIA _returnvalue isIA)
  (Variables|/Game/Blueprints/PODS/POD_PROTOTYPE.POD_PROTOTYPE_C|SetRespawnTransform _returnvalue respawnLocation)
  (Variables|/Game/Blueprints/PODS/POD_PROTOTYPE.POD_PROTOTYPE_C|SetCurrentLap _returnvalue (Variables|/Game/Blueprints/PODS/POD_PROTOTYPE.POD_PROTOTYPE_C|GetCurrentLap OldActor))
  (Variables|/Game/Blueprints/PODS/POD_PROTOTYPE.POD_PROTOTYPE_C|SetCurrentPosition _returnvalue (Variables|/Game/Blueprints/PODS/POD_PROTOTYPE.POD_PROTOTYPE_C|GetCurrentPosition OldActor))
  (Variables|/Game/Blueprints/PODS/POD_PROTOTYPE.POD_PROTOTYPE_C|SetPreviousCurrentPosition _returnvalue (Variables|/Game/Blueprints/PODS/POD_PROTOTYPE.POD_PROTOTYPE_C|GetPreviousCurrentPosition OldActor))
  (Variables|/Game/Blueprints/PODS/POD_PROTOTYPE.POD_PROTOTYPE_C|SetisFirstTime _returnvalue (Variables|/Game/Blueprints/PODS/POD_PROTOTYPE.POD_PROTOTYPE_C|GetisFirstTime OldActor))
  (Variables|/Game/Blueprints/PODS/POD_PROTOTYPE.POD_PROTOTYPE_C|SetUseAbilities _returnvalue (Variables|/Game/Blueprints/PODS/POD_PROTOTYPE.POD_PROTOTYPE_C|GetUseAbilities OldActor))
  (Variables|/Game/Blueprints/PODS/POD_PROTOTYPE.POD_PROTOTYPE_C|SetColorTrace _returnvalue (Variables|/Game/Blueprints/PODS/POD_PROTOTYPE.POD_PROTOTYPE_C|GetColorTrace OldActor))
  (Default|InitColorTrace _returnvalue)
  (Audio|PlaySoundatLocation "/Game/Sounds/SFX/respawn.respawn" (Math|Conversions|ToVector(Float) (Class|SkeletalMeshComponent|GetPosition (Variables|/Game/Blueprints/PODS/POD_PROTOTYPE.POD_PROTOTYPE_C|GetPOD_MESH _returnvalue))) "0, 0, 0" 1.0 1.0 0.0 0 0 0)
  (if (not (Variables|Default|GetUseIA))
    (Pawn|Possess (Variables|Default|GetPlayerControllerReference) _returnvalue)
    (bind _asmy_player_controller (Utilities|Casting|CastToMyPlayerController (Game|GetPlayerController 0)))
    (Variables|/Game/GameModes/MyPlayerController.MyPlayerController_C|SetPodReference _asmy_player_controller _returnvalue)))

(event EventTick
  (params (DeltaSeconds :type Float%20%28single-precision%29))
  ;[1 1 1] Event Tick
  (|CallParentFunction DeltaSeconds)
  (bind _ultfired (CallFunction|IAAbilitiesControl))
  (if (Variables|Default|GetUseIA)
    (if _ultfired
      (Utilities|FlowControl|Delay (Variables|Default|GetUltimateMaxTime))
      (CallFunction|ToggleInvisibility))))

(event EventTriggerAbility
  ;[1 1 1] Abilities Control
  (if (Variables|Default|GetUseAbilities)
    (if (Variables|Default|GetUseIA)
      (Utilities|FlowControl|Delay (Math|Float|Lerp 2.0 0.0 (Variables|Default|GetAbilityEfectiveness))))
    (CallFunction|FireMissile)))

(event EventTriggerUltimate
  ;[1 1 1] Abilities Control
  (if (Variables|Default|GetUseAbilities)
    (if (Variables|Default|GetUseIA)
      (Utilities|FlowControl|Delay (Math|Float|Lerp 2.0 0.0 (Variables|Default|GetUltEfectiveness))))
    (CallFunction|ToggleInvisibility)
    (Utilities|FlowControl|Delay (Variables|Default|GetUltimateMaxTime))
    (CallFunction|ToggleInvisibility)))

(fn ConstructionScript
  (|CallParentFunction))

(fn FireMissile
  (bind _missilespawnpoint (Variables|Default|GetMissileSpawnPoint))
  ;[1 1 1] Spawns missile and plays missile sound
  (Game|SpawnActorfromClass "/Game/Blueprints/Spawnables/MissileProjectile.MissileProjectile_C" (Math|Transform|MakeTransform (Transformation|GetWorldLocation _missilespawnpoint) (Math|Rotator|MakeRotator 0.0 0.0 (.yaw (Transformation|GetWorldRotation _missilespawnpoint)))) "Undefined" 0 0)
  (Audio|PlaySoundatLocation "/Game/VFX_Toolkit_V1/Sounds/SC_MissileLaunch.SC_MissileLaunch" (Transformation|GetWorldLocation (Variables|Default|GetMissileSpawnPoint)) "0, 0, 0" 1.0 1.0 0.0 0 0 0))

(fn ToggleInvisibility
  (bind _shipmesh (Variables|Default|GetShipMesh))
  (bind _returnvalue (Transformation|GetWorldLocation _shipmesh))
  (if (Variables|Default|GetisInvisible)
    (Rendering|Material|SetMaterial (Variables|Default|GetPOD_MESH) 0 (Variables|Default|GetInitialMaterialReference))
    (Audio|PlaySoundatLocation "/Game/Sounds/SFX/appear.appear" _returnvalue "0, 0, 0" 1.0 1.0 0.0 0 0 0)
    (else
      (Variables|Default|SetInitialMaterialReference (Rendering|Material|GetMaterial (Variables|Default|GetPOD_MESH) 0))
      (Rendering|Material|SetMaterial (Variables|Default|GetPOD_MESH) 0 "/Game/Materials/Stealth.Stealth")
      (Audio|PlaySoundatLocation "/Game/Sounds/SFX/disappear.disappear" _returnvalue "0, 0, 0" 1.0 1.0 0.0 0 0 0)))
  (CallFunction|ShowParticles (Variables|Default|GetisInvisible))
  (Variables|Default|SetisInvisible (not (Variables|Default|GetisInvisible))))

(fn IAAbilitiesControl
  (bind _stabilizationplane (Variables|Default|GetStabilizationPlane))
  (bind _returnvalue (Math|Vector|GetForwardVector _stabilizationplane))
  (bind (_x _y) (Math|Vector|BreakVector _returnvalue))
  (if (Variables|Default|GetUseAbilities)
    (LocalVariables|SetUltFired_ false)
    (LocalVariables|SetAbilityFired_ false)
    (if (Variables|Default|GetUseIA)
      (Utilities|FlowControl|Sequence
        (:then_0
          ;[1 1 1] Missile
          (if (not (Variables|Default|GetAbilityActive))
            (for _array_element (Variables|Default|GetOtherPods)
              (Utilities|IsValid _array_element
                (:Is%20Valid
                  (if (< (Math|Vector|VectorLength (- (Transformation|GetActorLocation _array_element) (Transformation|GetWorldLocation _stabilizationplane))) 2e+03)
                    (if (>= (Math|Float|Clamp(Float) (Math|Vector2D|DotProduct(2D) (Math|Vector2D|MakeVector2D (.X (Math|Vector|BreakVector (Math|Vector|Normalize (- (Transformation|GetActorLocation _array_element) (Transformation|GetWorldLocation _stabilizationplane))))) (.Y (Math|Vector|BreakVector (Math|Vector|Normalize (- (Transformation|GetActorLocation _array_element) (Transformation|GetWorldLocation _stabilizationplane)))))) (Math|Vector2D|MakeVector2D _x _y))) 0.9)
                      (Variables|Default|SetAbilityActive true)
                      (CallFunction|FireMissile)
                      (LocalVariables|SetAbilityFired_ true))))))))
        (:then_1
          ;[1 1 1] Invisibility
          (if (not (Variables|Default|GetUltimateActive))
            (bind _array_element_2 (Utilities|Array|ForEachLoopwithBreak (Variables|Default|GetOtherPods) :!label _label)
              (:LoopBody
                (Utilities|IsValid _array_element_2
                  (:Is%20Valid
                    (if (< (Math|Vector|VectorLength (- (Transformation|GetActorLocation _array_element_2) (Transformation|GetWorldLocation (Variables|Default|GetStabilizationPlane)))) 1e+03)
                      (Variables|Default|SetUltimateActive true)
                      (CallFunction|ToggleInvisibility)
                      (LocalVariables|SetUltFired_ true)
                      (goto _label Break))))))))
        (:then_2
          ;[1 1 1] Return bool values
          (return (LocalVariables|GetUltFired_) (LocalVariables|GetAbilityFired_)))))))