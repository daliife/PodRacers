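; Pod_C is a pod vehicle variant whose ability is a forward teleport with a shockwave, and its ultimate runs the same logic.
; A box trace limits the jump, which moves colliders and ship mesh between explosion effects, then radially impulses nearby physics bodies.
; AI pods trigger it when the forward dot product is high and no ability is active.
; Respawn spawns a fresh Pod_C, passing on target and AI state, and possesses it for human players.
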(event Collision|EventActorBeginOverlap
  (params (OtherActor :type Actor%20Object%20Reference)))

(event EventTick
  (params (DeltaSeconds :type Float%20%28single-precision%29))
  (|CallParentFunction DeltaSeconds)
  (if (Variables|Default|GetUseIA)
    (CallFunction|AIAbilityControl (Variables|Default|GetForwardDotProduct))))

(event EventBeginPlay
  (|CallParentFunction) ; This node is disabled and will not be called.\nDrag off pins to build functionality.
)

(event EventTriggerAbility
  (bind _stabilizationplane (Variables|Default|GetStabilizationPlane))
  (bind _tp_distance (Variables|Default|GetTP_Distance))
  (bind _returnvalue (Transformation|GetWorldLocation _stabilizationplane))
  (bind _returnvalue_2 (Math|Vector|GetForwardVector _stabilizationplane))
  (bind _returnvalue_3 (* _returnvalue_2 _tp_distance))
  (bind _returnvalue_4 (+ _returnvalue "0, 0,100.000000"))
  (bind (_outhit _returnvalue_5) (Collision|BoxTraceByChannel _returnvalue_4 (+ _returnvalue_4 _returnvalue_3) (.BoxExtent (Collision|GetActorBounds true)) (Transformation|GetWorldRotation _stabilizationplane) "TraceTypeQuery1" false 0 "ForDuration"))
  (Effects|SpawnEmitteratLocation "/Game/StarterContent/Particles/P_Explosion.P_Explosion" _returnvalue "0, 0, 0" "4.000000,4.000000,4.000000")
  (Transformation|AddWorldOffset (Variables|Default|GetRight_Sphere_Collider) (select _returnvalue_5 (- (.Location (Collision|BreakHitResult _outhit)) _returnvalue_4) _returnvalue_3) false true)
  (Effects|SpawnEmitteratLocation "/Game/StarterContent/Particles/P_Explosion.P_Explosion" _returnvalue "0, 0, 0" "4.000000,4.000000,4.000000")
  (Rendering|Debug|DrawDebugSphere _returnvalue 1e+03 12 "(R=1.000000,G=1.000000,B=1.000000,A=1.000000)" 5.0 1e+01)
  (bind _outcomponents (Collision|SphereOverlapComponents _returnvalue 1e+03 (Utilities|Array|MakeArray "ObjectTypeQuery4") 0 (Utilities|Array|MakeArray self)))
  (Physics|AddRadialImpulse _outcomponents _returnvalue 1e+03 1e+06 "RIF_Constant" false))

(event EventRespawn
  (params (respawnLocation :type Transform) (newTarget :type Actor%20Object%20Reference) (isIA :type Boolean))
  (bind (_location _rotation) (Math|Transform|BreakTransform respawnLocation))
  (bind _returnvalue (Game|SpawnActorfromClass "Pod_C_C" (Math|Transform|MakeTransform _location _rotation (Math|Vector|MakeVector 1.0 1.0 1.0)) "AdjustIfPossibleButAlwaysSpawn" 0 0))
  (Variables|/Game/Blueprints/PODS/POD_PROTOTYPE.POD_PROTOTYPE_C|SetUseIA _returnvalue isIA)
  (Variables|/Game/Blueprints/PODS/POD_PROTOTYPE.POD_PROTOTYPE_C|SetRespawnTransform _returnvalue respawnLocation)
  (Variables|/Game/Blueprints/PODS/POD_PROTOTYPE.POD_PROTOTYPE_C|SetTarget _returnvalue newTarget)
  (Audio|PlaySoundatLocation "/Game/Sounds/SFX/teleport.teleport" (Math|Conversions|ToVector(Float) (Class|SkeletalMeshComponent|GetPosition (Variables|/Game/Blueprints/PODS/POD_PROTOTYPE.POD_PROTOTYPE_C|GetPOD_MESH _returnvalue))) "0, 0, 0" 1.0 1.0 0.0 0 0 0)
  (if (not (Variables|/Game/Blueprints/PODS/POD_PROTOTYPE.POD_PROTOTYPE_C|GetUseIA _returnvalue))
    (Pawn|Possess (Variables|Default|GetPlayerControllerReference) _returnvalue)))

(event EventTriggerUltimate
  (bind _stabilizationplane (Variables|Default|GetStabilizationPlane))
  (bind _tp_distance (Variables|Default|GetTP_Distance))
  (bind _returnvalue (Transformation|GetWorldLocation _stabilizationplane))
  (bind _returnvalue_2 (Math|Vector|GetForwardVector _stabilizationplane))
  (bind _returnvalue_3 (* _returnvalue_2 _tp_distance))
  (bind _returnvalue_4 (+ _returnvalue "0, 0,100.000000"))
  (bind (_outhit _returnvalue_5) (Collision|BoxTraceByChannel _returnvalue_4 (+ _returnvalue_4 _returnvalue_3) (.BoxExtent (Collision|GetActorBounds true)) (Transformation|GetWorldRotation _stabilizationplane) "TraceTypeQuery1" false 0 "ForDuration"))
  (Effects|SpawnEmitteratLocation "/Game/StarterContent/Particles/P_Explosion.P_Explosion" _returnvalue "0, 0, 0" "4.000000,4.000000,4.000000")
  (Transformation|AddWorldOffset (Variables|Default|GetRight_Sphere_Collider) (select _returnvalue_5 (- (.Location (Collision|BreakHitResult _outhit)) _returnvalue_4) _returnvalue_3) false true)
  (Effects|SpawnEmitteratLocation "/Game/StarterContent/Particles/P_Explosion.P_Explosion" _returnvalue "0, 0, 0" "4.000000,4.000000,4.000000")
  (Rendering|Debug|DrawDebugSphere _returnvalue 1e+03 12 "(R=1.000000,G=1.000000,B=1.000000,A=1.000000)" 5.0 1e+01)
  (bind _outcomponents (Collision|SphereOverlapComponents _returnvalue 1e+03 (Utilities|Array|MakeArray "ObjectTypeQuery4") 0 (Utilities|Array|MakeArray self)))
  (Physics|AddRadialImpulse _outcomponents _returnvalue 1e+03 1e+06 "RIF_Constant" false))

(fn ConstructionScript
  (|CallParentFunction))

(fn AIAbilityControl
  (params (ForwardValue :type Float%20%28single-precision%29))
  (bind _playercontrollerreference (Variables|Default|GetPlayerControllerReference))
  (if (>= ForwardValue 0.9)
    (if (not (Variables|/Game/GameModes/MyPlayerController.MyPlayerController_C|GetAbilityActive _playercontrollerreference))
      (Variables|/Game/GameModes/MyPlayerController.MyPlayerController_C|SetAbilityActive _playercontrollerreference true)
      (CallFunction|TriggerAbility))))