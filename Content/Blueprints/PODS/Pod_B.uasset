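; Pod_B is a playable or AI-driven pod variant that loads its "POD_B" stats and specializes in defensive drops.
; Its ability spawns a mine behind the pod with a sound, and its ultimate spawns a barrier there.
; Respawn spawns a fresh Pod_B, carries over the AI flag and respawn transform, and has the player controller possess human pods.
; IAAbilityControl is empty, with its proximity and facing-check targeting logic left disconnected.
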(event Collision|EventActorBeginOverlap
  (params (OtherActor :type Actor%20Object%20Reference)))

(event EventRespawn
  (params (respawnLocation :type Transform) (isIA :type Boolean))
  (bind (_location _rotation) (Math|Transform|BreakTransform respawnLocation))
  (bind _returnvalue (Game|SpawnActorfromClass "Pod_B_C" (Math|Transform|MakeTransform _location _rotation (Math|Vector|MakeVector 1.0 1.0 1.0)) "AdjustIfPossibleButAlwaysSpawn" 0 0))
  (bind _output_get (Variables|/Game/Blueprints/PODS/POD_PROTOTYPE.POD_PROTOTYPE_C|SetUseIA _returnvalue isIA))
  (Variables|/Game/Blueprints/PODS/POD_PROTOTYPE.POD_PROTOTYPE_C|SetRespawnTransform _returnvalue respawnLocation)
  (Variables|/Game/Blueprints/PODS/POD_PROTOTYPE.POD_PROTOTYPE_C|SetTarget _returnvalue 0)
  (Audio|PlaySoundatLocation "/Game/Sounds/SFX/teleport.teleport" (Math|Conversions|ToVector(Float) (Class|SkeletalMeshComponent|GetPosition (Variables|/Game/Blueprints/PODS/POD_PROTOTYPE.POD_PROTOTYPE_C|GetPOD_MESH _returnvalue))) "0, 0, 0" 1.0 1.0 0.0 0 0 0)
  (if (not _output_get)
    (Pawn|Possess (Variables|Default|GetPlayerControllerReference) _returnvalue)))

(event EventTick
  (params (DeltaSeconds :type Float%20%28single-precision%29))
  (|CallParentFunction DeltaSeconds) ; This node is disabled and will not be called.\nDrag off pins to build functionality.
)

(event EventBeginPlay
  (|CallParentFunction)
  (CallFunction|InitStatsValues "POD_B"))

(event EventTriggerAbility
  (bind _stabilizationplane (Variables|Default|GetStabilizationPlane))
  ;[1 1 1] Spawns mine and plays mine sound
  (Game|SpawnActorfromClass "/Game/Blueprints/Spawnables/MineProjectile.MineProjectile_C" (Math|Transform|MakeTransform (- (+ (Transformation|GetWorldLocation _stabilizationplane) "0, 0,50.000000") (* (Math|Vector|GetForwardVector _stabilizationplane) 8e+02)) (Transformation|GetWorldRotation _stabilizationplane)) "AlwaysSpawn" 0 0)
  (Audio|PlaySoundatLocation "/Engine/VREditor/Sounds/UI/Camera_Shutter.Camera_Shutter" (Transformation|GetActorLocation) "0, 0, 0" 1.0 1.0 0.0 0 0 0))

(event EventTriggerUltimate
  (bind _stabilizationplane (Variables|Default|GetStabilizationPlane))
  (Game|SpawnActorfromClass "/Game/Blueprints/Spawnables/Barrier.Barrier_C" (Math|Transform|MakeTransform (- (Transformation|GetWorldLocation _stabilizationplane) (* (Math|Vector|GetForwardVector _stabilizationplane) 8e+02)) (Transformation|GetWorldRotation _stabilizationplane)) "AlwaysSpawn" 0 0))

(fn ConstructionScript
  (|CallParentFunction))

(fn IAAbilityControl)