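; Physics-driven pod vehicle, steered by setting strengths on a forward thruster and four front and back turn thrusters from input axes.
; Turbo and Brake flip on press and release to boost forward thrust or raise body linear damping.
; Look axes and mouse wheel rotate and zoom the spring-arm camera.
; SetSupportLocations line-traces from a constraint to place its support on the hit or at full extent, updating ground contact.
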(event Input|ActionEvents|InputActionBrake
  (params (Key :type Key%20Structure))
  (:Pressed
    (Utilities|FlowControl|FlipFlop :!label _label
      (:A
        (Class|PrimitiveComponent|SetLinearDamping (Variables|Default|GetMainBody) 1.0))
      (:B
        (Class|PrimitiveComponent|SetLinearDamping (Variables|Default|GetMainBody) 0.1))))
  (:Released
    (goto _label)))

(event Input|ActionEvents|InputActionTurbo
  (params (Key :type Key%20Structure))
  (:Pressed
    (Utilities|FlowControl|FlipFlop :!label _label
      (:A
        (Variables|Default|SetThrustForwardBoost 4.0))
      (:B
        (Variables|Default|SetThrustForwardBoost 1.0))))
  (:Released
    (goto _label)))

(event Input|AxisEvents|InputAxisMoveForward
  (params (AxisValue :type Float%20%28single-precision%29))
  (Variables|/Script/Engine.PhysicsThrusterComponent|SetThrustStrength (Variables|Default|GetForwardThrust) (* AxisValue (* (Variables|Default|GetThrustForwardForce) (Variables|Default|GetThrustForwardBoost)))))

(event Input|AxisEvents|InputAxisMoveRight
  (params (AxisValue :type Float%20%28single-precision%29))
  (bind _returnvalue (* AxisValue 1e+05))
  (bind _returnvalue_2 (Math|Float|Absolute(Float) _returnvalue))
  (if (== AxisValue 0.0)
    (Variables|/Script/Engine.PhysicsThrusterComponent|SetThrustStrength (Variables|Default|GetLeftTurnThrust) 0.0)
    (Variables|/Script/Engine.PhysicsThrusterComponent|SetThrustStrength (Variables|Default|GetRightTurnThrust) 0.0)
    (Variables|/Script/Engine.PhysicsThrusterComponent|SetThrustStrength (Variables|Default|GetRightBackTurnThrust) 0.0)
    (Variables|/Script/Engine.PhysicsThrusterComponent|SetThrustStrength (Variables|Default|GetLeftBackTurnThrust) 0.0)
    (elif (> _returnvalue 0.0)
      (Variables|/Script/Engine.PhysicsThrusterComponent|SetThrustStrength (Variables|Default|GetLeftTurnThrust) _returnvalue_2)
      (Variables|/Script/Engine.PhysicsThrusterComponent|SetThrustStrength (Variables|Default|GetRightBackTurnThrust) _returnvalue_2)
      (else
        (Variables|/Script/Engine.PhysicsThrusterComponent|SetThrustStrength (Variables|Default|GetRightTurnThrust) _returnvalue_2)
        (Variables|/Script/Engine.PhysicsThrusterComponent|SetThrustStrength (Variables|Default|GetLeftBackTurnThrust) _returnvalue_2)))))

(event Input|AxisEvents|InputAxisTurnRate
  (params (AxisValue :type Float%20%28single-precision%29))
  (Transformation|AddRelativeRotation (Variables|Default|GetSpringArm) (Math|Rotator|MakeRotator 0.0 0.0 (* AxisValue (Variables|Default|GetCameraVelocity))) false false))

(event Input|AxisEvents|InputAxisLookUpRate
  (params (AxisValue :type Float%20%28single-precision%29))
  (Transformation|AddRelativeRotation (Variables|Default|GetSpringArm) (Math|Rotator|MakeRotator 0.0 (* AxisValue (Variables|Default|GetCameraVelocity)) 0.0) false false))

(event Input|MouseEvents|MouseWheelAxis
  (params (AxisValue :type Float%20%28single-precision%29))
  (bind _springarm (Variables|Default|GetSpringArm))
  (Variables|/Script/Engine.SpringArmComponent|SetTargetArmLength _springarm (+ (* AxisValue -5.0) (Variables|/Script/Engine.SpringArmComponent|GetTargetArmLength _springarm))))

(fn ConstructionScript)

(fn SetSupportLocations
  (params (Constraint :type Physics%20Constraint%20Component%20Object%20Reference) (Support :type Static%20Mesh%20Component%20Object%20Reference) (prevTouchingGround :type Boolean) (DownVector :type Vector))
  (bind _returnvalue (Transformation|GetWorldLocation Constraint))
  (bind _returnvalue_2 (- _returnvalue DownVector))
  (bind (_outhit _returnvalue_3) (Collision|LineTraceByChannel _returnvalue _returnvalue_2 "TraceTypeQuery1" false 0 "None" true "(R=1.000000,G=0.000000,B=0.000000,A=1.000000)" "(R=0.000000,G=1.000000,B=0.000000,A=1.000000)" 0.1))
  (if _returnvalue_3
    (Transformation|SetWorldLocation Support (.Location (Collision|BreakHitResult _outhit)) false false)
    (return prevTouchingGround DownVector)
    (else
      (Transformation|SetWorldLocation Support _returnvalue_2 false false)
      (return false DownVector))))